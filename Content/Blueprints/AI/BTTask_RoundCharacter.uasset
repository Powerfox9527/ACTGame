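; Behavior tree task that makes an AGCharacterBase pawn shift sideways to a random spot.
; It finishes successfully at once if the character is playing a montage.
; Otherwise AIMoveTo targets the mesh location plus a random left or right offset along the actor's right vector, with a loose acceptance radius.
; Only move success finishes the task on that path; move failure and a failed cast never call FinishExecute.
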(event EventReceiveExecuteAI
  (params (OwnerController :type AI%20Controller%20Object%20Reference) (ControlledPawn :type Pawn%20Object%20Reference))
  (bind _asagcharacter_base (Utilities|Casting|CastToAGCharacterBase ControlledPawn))
  (bind _returnvalue (Class|AGCharacterBase|IsPlayingMontage _asagcharacter_base))
  (if _returnvalue
    (AI|BehaviorTree|FinishExecute true)
    (else
      (AI|AIMoveTo _asagcharacter_base (+ (Transformation|GetWorldLocation (Variables|/Script/Engine.Character|GetMesh _asagcharacter_base)) (* (Transformation|GetActorRightVector _asagcharacter_base) (Math|Random|RandomFloatinRange -5e+02 5e+02))) 0 2e+02 false
        (:OnSuccess
          (AI|BehaviorTree|FinishExecute true))))))

(event EventTick
  (params (OwnerActor :type Actor%20Object%20Reference) (DeltaSeconds :type Float%20%28single-precision%29)))
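; AGP_SmallIce is a small ice projectile that damages characters through the Gameplay Ability System.
; When its capsule overlaps an AGCharacterBase other than the owning character, it applies its damage effect spec to that character's ability system component.
; It then spawns an ice hit particle at its location and destroys itself after a brief delay.
; Overlaps with the owner or other actor types are ignored.
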(event OnComponentBeginOverlap(CapsuleComponent)
  (params (OverlappedComponent :type Primitive%20Component%20Object%20Reference) (OtherActor :type Actor%20Object%20Reference) (OtherComp :type Primitive%20Component%20Object%20Reference) (OtherBodyIndex :type Integer) (bFromSweep :type Boolean) (SweepResult :type Hit%20Result%20Structure%20%28by%20ref%29))
  (if (not (== OtherActor (Variables|Default|GetOwningCharacter)))
    (bind _asagcharacter_base (Utilities|Casting|CastToAGCharacterBase OtherActor))
    (GameplayEffects|ApplyGameplayEffectSpecToSelf (Variables|/Script/ACTGame.AGCharacterBase|GetAbilitySystemComponent _asagcharacter_base) (Variables|Default|GetDamageEffectSpecHandle))
    (Effects|SpawnEmitteratLocation "/Game/Particles/AdvancedMagicFX12/particles/P_ky_hit_ice.P_ky_hit_ice" (Transformation|GetActorLocation))
    (Utilities|FlowControl|Delay 0.1)
    (Actor|DestroyActor)))

(event EventBeginPlay)

(event Collision|EventActorBeginOverlap
  (params (OtherActor :type Actor%20Object%20Reference)))

(fn ConstructionScript)
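; BP_NatPlayer is a player Blueprint that activates Gameplay Ability System abilities in response to UI requests.
; On BeginPlay it gets BP_GameMode and binds a handler to the ActivateAbility event on its MainView.
; The handler matches the received ability name against the display names of the CharacterAbilities classes and tries to activate matches through the AbilitySystemComponent, allowing remote activation.
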(event Custom|CustomEvent_0
  (params (AbilityName :type Text))
  (for _array_element (Variables|Default|GetCharacterAbilities)
    (if (Utilities|Enum|Equal(Enum) AbilityName (Utilities|Text|ToText(String) (Utilities|GetClassDisplayName _array_element)))
      (Abilities|TryActivateAbilitybyClass (Variables|Default|GetAbilitySystemComponent) _array_element true))))

(event EventBeginPlay
  (bind _asbp_game_mode (Utilities|Casting|CastToBP_GameMode (Game|GetGameMode)))
  (EventDispatchers|BindEventtoActivateAbility (Variables|/Game/Blueprints/BP_GameMode.BP_GameMode_C|GetMainView _asbp_game_mode) (delegate Custom|CustomEvent_0)))

(event Collision|EventActorBeginOverlap
  (params (OtherActor :type Actor%20Object%20Reference)))

(event EventTick
  (params (DeltaSeconds :type Float%20%28single-precision%29)))

(fn ConstructionScript)
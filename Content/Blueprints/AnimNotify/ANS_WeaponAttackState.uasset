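; Anim notify state that marks the window in an animation during which a character's weapon can attack.
; On begin it casts the mesh owner to AGCharacterBase and sets the weapon's CanAttack flag to true.
; On end it sets the flag back to false, and owners of other classes are ignored.
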(fn ReceivedNotifyBegin
  (params (MeshComp :type Skeletal%20Mesh%20Component%20Object%20Reference) (Animation :type Anim%20Sequence%20Base%20Object%20Reference) (TotalDuration :type Float%20%28single-precision%29))
  (bind _asagcharacter_base (Utilities|Casting|CastToAGCharacterBase (Components|GetOwner MeshComp)))
  (Variables|/Script/ACTGame.WeaponActor|SetCanAttack (Variables|/Script/ACTGame.AGCharacterBase|GetWeapon _asagcharacter_base) true)
  (return true))

(fn ReceivedNotifyEnd
  (params (MeshComp :type Skeletal%20Mesh%20Component%20Object%20Reference) (Animation :type Anim%20Sequence%20Base%20Object%20Reference))
  (bind _asagcharacter_base (Utilities|Casting|CastToAGCharacterBase (Components|GetOwner MeshComp)))
  (Variables|/Script/ACTGame.WeaponActor|SetCanAttack (Variables|/Script/ACTGame.AGCharacterBase|GetWeapon _asagcharacter_base) false)
  (return true))
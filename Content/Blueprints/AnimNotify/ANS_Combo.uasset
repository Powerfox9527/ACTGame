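; Anim notify state that marks a combo window in an animation by setting the owning character's next combo section name.
; On begin, it casts the mesh owner to ACTGameCharacter and sets ComboSectionName to a random entry from ComboSectionNames.
; On end, it resets that name to None, but casts to the more specific BP_NatPlayer, so the reset applies only to owners of that class.
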(fn ReceivedNotifyBegin
  (params (MeshComp :type Skeletal%20Mesh%20Component%20Object%20Reference) (Animation :type Anim%20Sequence%20Base%20Object%20Reference) (TotalDuration :type Float%20%28single-precision%29))
  (bind _asactgame_character (Utilities|Casting|CastToACTGameCharacter (Components|GetOwner MeshComp)))
  (Utilities|IsValid _asactgame_character
    (:Is%20Valid
      (Variables|/Script/ACTGame.ACTGameCharacter|SetComboSectionName _asactgame_character (.OutItem (Utilities|Array|Random (Variables|Default|GetComboSectionNames))))
      (return false))))

(fn ReceivedNotifyEnd
  (params (MeshComp :type Skeletal%20Mesh%20Component%20Object%20Reference) (Animation :type Anim%20Sequence%20Base%20Object%20Reference))
  (bind _asbp_nat_player (Utilities|Casting|CastToBP_NatPlayer (Components|GetOwner MeshComp)))
  (Utilities|IsValid _asbp_nat_player
    (:Is%20Valid
      (Variables|/Script/ACTGame.ACTGameCharacter|SetComboSectionName _asbp_nat_player "None")
      (return false))))
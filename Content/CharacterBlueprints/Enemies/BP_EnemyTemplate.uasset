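; Base enemy character Blueprint that drives a status widget and keeps the enemy facing its hate target.
; On BeginPlay it registers async Ability System attribute listeners for health and break changes.
; Their callbacks set the EnemyStatus widget's bars, scaling health by base MaxHealth and passing break through directly.
; Each Tick it reads HateCharacter from the Blackboard and rotates toward that actor without roll.
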(event Custom|HealthChangeEvent
  (params (Attribute :type Gameplay%20Attribute%20Structure) (NewValue :type Float%20%28single-precision%29) (OldValue :type Float%20%28single-precision%29))
  (CallFunction|ChangeUIHealth NewValue))

(event Custom|BreakChangeEvent
  (params (Attribute :type Gameplay%20Attribute%20Structure) (NewValue :type Float%20%28single-precision%29) (OldValue :type Float%20%28single-precision%29))
  (CallFunction|ChangeUIBreak NewValue))

(event EventBeginPlay
  (bind _abilitysystemcomponent (Variables|Default|GetAbilitySystemComponent))
  (|CallParentFunction)
  (bind _asynctaskproxy (|ListenforAttributeChange _abilitysystemcomponent "(AttributeName=\"Health\",Attribute=/Script/ACTGame.AGAttributeSet:Health,AttributeOwner=None)")
    (:then
      (EventDispatchers|BindEventtoOnAttributeChanged _asynctaskproxy (delegate Custom|HealthChangeEvent))
      (bind _asynctaskproxy_2 (|ListenforAttributeChange _abilitysystemcomponent "(AttributeName=\"Break\",Attribute=/Script/ACTGame.AGAttributeSet:Break,AttributeOwner=None)")
        (:then
          (EventDispatchers|BindEventtoOnAttributeChanged _asynctaskproxy_2 (delegate Custom|BreakChangeEvent)))))))

(event EventTick
  (params (DeltaSeconds :type Float%20%28single-precision%29))
  (bind _asactor (Utilities|Casting|CastToActor (AI|Components|Blackboard|GetValueasObject (AI|GetBlackboard 0) (Utilities|Name|MakeLiteralName "HateCharacter"))))
  (Class|AGCharacterBase|RotatetoActor _asactor true))

(fn ConstructionScript)

(fn ChangeUIHealth
  (params (NewValue :type Float%20%28single-precision%29))
  (bind _asenemy_status (Utilities|Casting|CastToEnemyStatus (UserInterface|GetWidget (Variables|Default|GetEnemyStatus))))
  (Utilities|IsValid _asenemy_status
    (:Is%20Valid
      (Progress|SetPercent (Variables|/Game/Blueprints/UI/EnemyStatus.EnemyStatus_C|GetHealth _asenemy_status) (/ NewValue (.BaseValue (Utilities|Struct|BreakGameplayAttributeData (Variables|/Script/ACTGame.AGAttributeSet|GetMaxHealth (Variables|Default|GetAttributeSet)))))))))

(fn ChangeUIBreak
  (params (NewValue :type Float%20%28single-precision%29))
  (bind _asenemy_status (Utilities|Casting|CastToEnemyStatus (UserInterface|GetWidget (Variables|Default|GetEnemyStatus))))
  (Utilities|IsValid _asenemy_status
    (:Is%20Valid
      (Progress|SetPercent (Variables|/Game/Blueprints/UI/EnemyStatus.EnemyStatus_C|GetBreak _asenemy_status) NewValue))))